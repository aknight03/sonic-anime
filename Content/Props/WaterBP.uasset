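; Water volume prop that slows the third-person character and boosts its jump while inside a box trigger.
; On overlap it divides walk speed and raises jump velocity, then multiplies speed back and restores a fixed jump value on exit.
; It creates a WaterHUD widget at BeginPlay, and Tick shows or hides it by checking the WaterDivision value set by the overlap events.
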(event `self.Box.OnComponentBeginOverlap`
  (params (OverlappedComponent :type "PrimitiveComponent Object Reference") (OtherActor :type "Actor Object Reference") (OtherComp :type "PrimitiveComponent Object Reference") (OtherBodyIndex :type Integer) (bFromSweep :type Boolean) (SweepResult :type "HitResult Structure (by ref)"))
  (bind _asthird_person_character (cast `/Game/ThirdPersonBP/Blueprints/ThirdPersonCharacter` OtherActor))
  (set `self.WaterDivision` 4.0)
  (bind _charactermovement (`Character.CharacterMovement` _asthird_person_character))
  (set `CharacterMovementComponent.MaxWalkSpeed` (/ (`CharacterMovementComponent.MaxWalkSpeed` _charactermovement) 4.0) _charactermovement)
  (set `CharacterMovementComponent.JumpZVelocity` 1200.0 _charactermovement))

(event `self.Box.OnComponentEndOverlap`
  (params (OverlappedComponent :type "PrimitiveComponent Object Reference") (OtherActor :type "Actor Object Reference") (OtherComp :type "PrimitiveComponent Object Reference") (OtherBodyIndex :type Integer))
  (bind _asthird_person_character (cast `/Game/ThirdPersonBP/Blueprints/ThirdPersonCharacter` OtherActor))
  (set `self.WaterDivision` 1.0)
  (bind _charactermovement (`Character.CharacterMovement` _asthird_person_character))
  (set `CharacterMovementComponent.MaxWalkSpeed` (* (`CharacterMovementComponent.MaxWalkSpeed` _charactermovement) 4.0) _charactermovement)
  (set `CharacterMovementComponent.JumpZVelocity` 600.0 _charactermovement))

(event `self.ReceiveBeginPlay`
  (bind _returnvalue (`|CreateWidget` "/Game/hud/WaterHUD.WaterHUD_C"))
  (`UserWidget.AddToViewport` _returnvalue 0))

(event `self.ReceiveTick`
  (params (DeltaSeconds :type "Float (single-precision)"))
  (if (== (`self.WaterDivision`) 4.0)
    (`Widget.SetVisibility` (stale `self.ReceiveBeginPlay` _returnvalue) "Visible")
    (else
      (`Widget.SetVisibility` (stale `self.ReceiveBeginPlay` _returnvalue) "Hidden"))))

(fn `UserConstructionScript`)